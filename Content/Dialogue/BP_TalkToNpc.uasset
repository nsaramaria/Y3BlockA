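; BP_TalkToNpc is a simple NPC dialogue Blueprint that shows one line of dialogue per Talk event.
; Talk increments TalkIndex, then prints that entry of the Dialogue array with Print String while the index is in range.
; The index advances before the read and is never reset here, so calls past the last line print nothing.
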(event `/Game/Dialogue/BPI_Dialogue.Talk`
  (`/Engine/EditorBlueprintResources/StandardMacros.IncrementInt` (`self.TalkIndex`)
    (:`  `
      (if (< (`self.TalkIndex`) (`KismetArrayLibrary.Array_Length` (`self.dialogue`)))
        (`KismetSystemLibrary.PrintString` (`|GetArrayItem` (`self.dialogue`) (`self.TalkIndex`)))))))

(fn `UserConstructionScript`)